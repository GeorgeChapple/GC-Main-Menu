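; Blueprint actor that fades a 3D text component by animating its material transparency.
; On BeginPlay it creates a dynamic instance of the front material, assigns it to all four text faces, and sets the LerpScript easing to OutQuad.
; Every Tick it writes the X value of LerpScript's lerp vector into the material's Transparency parameter, so LerpScript drives the fade.
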(event EventBeginPlay
  (bind _text3d (Variables|Default|GetText3D))
  ;[1 1 1] Create dynamic material instance
  (bind _returnvalue (Rendering|Material|CreateDynamicMaterialInstance (Variables|/Script/Text3D.Text3DComponent|GetFrontMaterial (Variables|Default|GetText3D)) "None" "None" :!class /Script/Engine.KismetMaterialLibrary))
  (bind _output_get (Variables|Default|SetMat _returnvalue))
  (bind _output_get_2 (Variables|/Script/Text3D.Text3DComponent|SetFrontMaterial _text3d _output_get))
  (bind _output_get_3 (Variables|/Script/Text3D.Text3DComponent|SetBevelMaterial _text3d _output_get_2))
  (bind _output_get_4 (Variables|/Script/Text3D.Text3DComponent|SetExtrudeMaterial _text3d _output_get_3))
  (Variables|/Script/Text3D.Text3DComponent|SetBackMaterial _text3d _output_get_4)
  ;[1 1 1] Set lerp easing
  (Variables|/Script/MainMenu.LerpScript|Setease (Variables|Default|GetLerpScript) "outQuad"))

(event EventTick
  (params (DeltaSeconds :type Float%20%28single-precision%29))
  ;[1 1 1] Change transparency of material with lerp value
  (Rendering|Material|SetScalarParameterValue (Variables|Default|GetMat) "Transparency" (.x (Variables|/Script/MainMenu.LerpScript|GetlerpVector (Variables|Default|GetLerpScript))) :!class /Script/Engine.MaterialInstanceDynamic))

(fn ConstructionScript)