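; 3D menu text actor that rocks back and forth by rotating between a start and an end rotation.
; BeginPlay sets the start rotation and an InOutQuad ease on its LerpScript.
; Each Tick applies the lerp vector as the actor rotation and, whenever a lerp finishes, starts a new one toward the opposite end, toggled by ChooseLerp.
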(event EventTick
  (params (DeltaSeconds :type Float%20%28single-precision%29))
  (bind _returnvalue (Transformation|GetActorRotation))
  (bind _returnvalue_2 (Transformation|GetActorRotation))
  (bind _lerpscript (Variables|Default|GetLerpScript))
  (bind _lerpvector (Variables|/Script/MainMenu.LerpScript|GetlerpVector _lerpscript))
  ;[1 1 1] Set actor rotation based on lerp vector.
  (Transformation|SetActorRotation (Math|Rotator|MakeRotator (.x _lerpvector) (.y _lerpvector) (.z _lerpvector)) true)
  ;[1 1 1] Lerps vector, used to make text rock back and forth.
  (if (not (Variables|/Script/MainMenu.LerpScript|Getlerping (Variables|Default|GetLerpScript)))
    (if (Variables|Lerp|GetChooseLerp)
      (Class|LerpScript|StartLerp (Variables|Default|GetLerpScript) (Math|Vector|MakeVector (.roll _returnvalue_2) (.pitch _returnvalue_2) (.yaw _returnvalue_2)) (Variables|Lerp|GetEndRotateVal) (Variables|lerp|GetLerpTime))
      (Variables|Lerp|SetChooseLerp false)
      (else
        (Class|LerpScript|StartLerp (Variables|Default|GetLerpScript) (Math|Vector|MakeVector (.roll _returnvalue) (.pitch _returnvalue) (.yaw _returnvalue)) (Variables|lerp|GetStartRotateVal) (Variables|lerp|GetLerpTime))
        (Variables|Lerp|SetChooseLerp true)))))

(event EventBeginPlay
  (bind _startrotateval (Variables|lerp|GetStartRotateVal))
  ;[1 1 1] Set actor rotation to start vector on begin.
  (Transformation|SetActorRotation (Math|Rotator|MakeRotator (.x _startrotateval) (.y _startrotateval) (.z _startrotateval)))
  ;[1 1 1] Set lerp ease
  (Variables|/Script/MainMenu.LerpScript|Setease (Variables|Default|GetLerpScript) "inOutQuad"))

(fn ConstructionScript)