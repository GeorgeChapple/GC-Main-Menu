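; A clickable 3D menu object that shows a text label on hover and moves the player to a set position when clicked.
; Hover starts eased LerpScript tweens that grow or shrink the actor, with Tick applying the lerped scale.
; The same hover events drive the 3DTextFade child actor's LerpScript to fade its label in and out.
; Clicking lerps MyPlayer's location through the player's own LerpScript, with sounds on hover and click.
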(event MouseInput|EventActorOnClicked
  (params (ButtonPressed :type Key%20Structure :default "None"))
  (bind _player (Variables|Default|GetPlayer))
  (bind _returnvalue (Transformation|GetActorLocation _player))
  ;[1 1 1] Starts lerp to move
  (Class|LerpScript|StartLerp (Variables|/Game/Blueprints/MyPlayer.MyPlayer_C|GetLerpScript (Variables|Default|GetPlayer)) _returnvalue (Variables|PlayerLerp|GetSendPlayerToPos) (Variables|LerpTime|GetmoveLerpTimeToTake))
  ;[1 1 1] Play sound on click
  (Audio|PlaySoundatLocation (Variables|SoundEffect|GetSound) _returnvalue "0, 0, 0" 1.0 1.0 0.0 0 0 0 0))

(event EventTick
  (params (DeltaSeconds :type Float%20%28single-precision%29))
  ;[1 1 1] Manage object scale
  (Transformation|SetActorScale3D (Variables|/Script/MainMenu.LerpScript|GetlerpVector (Variables|Default|GetLerpScript))))

(event EventBeginPlay
  ;[1 1 1] Manage object scale
  (Variables|Default|Setrotate true)
  (Variables|/Script/MainMenu.LerpScript|SetlerpVector (Variables|Default|GetLerpScript) (Transformation|GetActorScale3D))
  ;[1 1 1] Get player actor
  (bind _outactors (Actor|GetAllActorsOfClass "/Game/Blueprints/MyPlayer.MyPlayer_C"))
  (bind _output_get (Variables|Default|SetOut%20Actors _outactors))
  (Variables|Default|SetPlayer (Utilities|Array|Get(acopy) _output_get))
  ;[1 1 1] Get lerp script from child
  (bind _as3dtext_fade (Utilities|Casting|CastTo3DTextFade (Variables|/Script/Engine.ChildActorComponent|GetChildActor (Variables|Default|Get3DTextFade))))
  (Variables|Default|SetChildLerpScript (Variables|/Game/Blueprints/3DTextFade.3DTextFade_C|GetLerpScript _as3dtext_fade))
  ;[1 1 1] Set text
  (bind _as3dtext_fade_2 (Utilities|Casting|CastTo3DTextFade (Variables|/Script/Engine.ChildActorComponent|GetChildActor (Variables|Default|Get3DTextFade))))
  (Variables|/Script/Text3D.Text3DComponent|SetText (Variables|/Game/Blueprints/3DTextFade.3DTextFade_C|GetText3D _as3dtext_fade_2) (Utilities|Text|ToText(String) (Variables|Text|GetText)))
  ;[1 1 1] Set Material
  (Rendering|Material|SetMaterial (Variables|Default|GetSphere) 0 (Variables|Material|GetMaterial))
  ;[1 1 1] Set lerp easing
  (Variables|/Script/MainMenu.LerpScript|Setease (Variables|Default|GetLerpScript) "outQuad"))

(event MouseInput|EventActorBeginCursorOver
  (bind _sizelerptimetotake (Variables|LerpTime|GetsizeLerpTimeToTake))
  (bind _childlerpscript (Variables|Default|GetChildLerpScript))
  ;[1 1 1] Grow lerp
  (Class|LerpScript|StartLerp (Variables|Default|GetLerpScript) (Transformation|GetActorScale3D) (Variables|SizeLerp|GetlerpPos2) _sizelerptimetotake)
  ;[1 1 1] Lerp text transparency 1
  (Class|LerpScript|StartLerp _childlerpscript (Variables|/Script/MainMenu.LerpScript|GetlerpVector _childlerpscript) "1.000000,0.000000,0.000000" _sizelerptimetotake)
  ;[1 1 1] Play sound on hover
  (Audio|PlaySoundatLocation "/Game/Sounds/Hover_Cue.Hover_Cue" (Transformation|GetActorLocation (Game|GetPlayerController 0)) "0, 0, 0" 1.0 1.0 0.0 0 0 0 0))

(event MouseInput|EventActorEndCursorOver
  (bind _childlerpscript (Variables|Default|GetChildLerpScript))
  (bind _sizelerptimetotake (Variables|LerpTime|GetsizeLerpTimeToTake))
  ;[1 1 1] Shrink lerp
  (Class|LerpScript|ForceLerpEnd (Variables|Default|GetLerpScript))
  (Class|LerpScript|StartLerp (Variables|Default|GetLerpScript) (Transformation|GetActorScale3D) (Variables|SizeLerp|GetlerpPos1) _sizelerptimetotake)
  ;[1 1 1] Lerp text transparency 0
  (Class|LerpScript|ForceLerpEnd _childlerpscript)
  (Class|LerpScript|StartLerp _childlerpscript (Variables|/Script/MainMenu.LerpScript|GetlerpVector _childlerpscript) "-0.050000,0.000000,0.000000" _sizelerptimetotake))

(fn ConstructionScript)