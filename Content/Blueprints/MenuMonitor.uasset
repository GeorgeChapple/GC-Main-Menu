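; Menu monitor actor that continuously sways in position and rotation while its screen colour cycles between two values.
; BeginPlay turns offsets into start and end targets relative to the placed transform and puts a dynamic screen material on the cube.
; Three eased lerp components drive location, rotation (via X-axis direction vector) and material colour.
; Tick applies their values and restarts each finished lerp in the opposite direction, creating independent ping-pong loops.
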(event EventTick
  (params (DeltaSeconds :type Float%20%28single-precision%29))
  (bind _lerpscriptc (Variables|ColourLerp|GetLerpScriptC))
  (bind _lerpvector (Variables|/Script/MainMenu.LerpScript|GetlerpVector _lerpscriptc))
  ;[1 1 1] Update attributes based on lerp vectors
  (Transformation|SetActorLocationAndRotation (Variables|/Script/MainMenu.LerpScript|GetlerpVector (Variables|PositionLerp|GetLerpScriptP)) (Math|Conversions|RotationFromXVector (Variables|/Script/MainMenu.LerpScript|GetlerpVector (Variables|RotationLerp|GetLerpScriptR))) false true)
  (Rendering|Material|SetVectorParameterValue (Variables|ColourLerp|GetScreenMaterialInstance) "Colour" (Utilities|Struct|MakeLinearColor (.x _lerpvector) (.y _lerpvector) (.z _lerpvector) 1.0) :!class /Script/Engine.MaterialInstanceDynamic)
  ;[1 1 1] Try and select rotation lerp
  (if (Variables|/Script/MainMenu.LerpScript|Getlerping (Variables|RotationLerp|GetLerpScriptR))
    _
    (elif (Variables|RotationLerp|GetChooseLerpR)
      (Class|LerpScript|StartLerp (Variables|RotationLerp|GetLerpScriptR) (Math|Rotator|GetRotationXVector (Transformation|GetActorRotation)) (Variables|RotationLerp|GetEndValR) (Variables|RotationLerp|GetLerpTimeR))
      (Variables|RotationLerp|SetChooseLerpR false)
      (else
        (Class|LerpScript|StartLerp (Variables|RotationLerp|GetLerpScriptR) (Math|Rotator|GetRotationXVector (Transformation|GetActorRotation)) (Variables|RotationLerp|GetStartValR) (Variables|RotationLerp|GetLerpTimeR))
        (Variables|RotationLerp|SetChooseLerpR true))))
  ;[1 1 1] Try and select position lerp
  (if (Variables|/Script/MainMenu.LerpScript|Getlerping (Variables|PositionLerp|GetLerpScriptP))
    _
    (elif (Variables|PositionLerp|GetChooseLerpP)
      (Class|LerpScript|StartLerp (Variables|PositionLerp|GetLerpScriptP) (Transformation|GetActorLocation) (Variables|PositionLerp|GetEndValP) (Variables|PositionLerp|GetLerpTimeP))
      (Variables|PositionLerp|SetChooseLerpP false)
      (else
        (Class|LerpScript|StartLerp (Variables|PositionLerp|GetLerpScriptP) (Transformation|GetActorLocation) (Variables|PositionLerp|GetStartValP) (Variables|PositionLerp|GetLerpTimeP))
        (Variables|PositionLerp|SetChooseLerpP true))))
  ;[1 1 1] Try and select colour lerp
  (if (not (Variables|/Script/MainMenu.LerpScript|Getlerping (Variables|ColourLerp|GetLerpScriptC)))
    (if (Variables|ColourLerp|GetChooseLerpC)
      (Class|LerpScript|StartLerp (Variables|ColourLerp|GetLerpScriptC) (Variables|ColourLerp|GetStartValC) (Variables|ColourLerp|GetEndValC) (Variables|ColourLerp|GetLerpTimeC))
      (Variables|ColourLerp|SetChooseLerpC false)
      (else
        (Class|LerpScript|StartLerp (Variables|ColourLerp|GetLerpScriptC) (Variables|ColourLerp|GetEndValC) (Variables|ColourLerp|GetStartValC) (Variables|ColourLerp|GetLerpTimeC))
        (Variables|ColourLerp|SetChooseLerpC true)))))

(event EventBeginPlay
  ;[1 1 1] Set position lerp vector to actor location, prevents lerping from 0,0,0 as soon as game starts.
  (Variables|/Script/MainMenu.LerpScript|SetlerpVector (Variables|PositionLerp|GetLerpScriptP) (Transformation|GetActorLocation))
  ;[1 1 1] Use vector values to determine start and end points based on actor location and rotation.
  (Variables|PositionLerp|SetStartValP (+ (Transformation|GetActorLocation) (Variables|PositionLerp|GetStartValP)))
  (Variables|PositionLerp|SetEndValP (+ (Transformation|GetActorLocation) (Variables|PositionLerp|GetEndValP)))
  (Variables|RotationLerp|SetStartValR (+ (Math|Rotator|GetRotationXVector (Transformation|GetActorRotation)) (Variables|RotationLerp|GetStartValR)))
  (Variables|RotationLerp|SetEndValR (+ (Math|Rotator|GetRotationXVector (Transformation|GetActorRotation)) (Variables|RotationLerp|GetEndValR)))
  ;[1 1 1] Set lerp easings
  (Variables|/Script/MainMenu.LerpScript|Setease (Variables|PositionLerp|GetLerpScriptP) "inOutQuad")
  (Variables|/Script/MainMenu.LerpScript|Setease (Variables|RotationLerp|GetLerpScriptR) "inOutQuad")
  (Variables|/Script/MainMenu.LerpScript|Setease (Variables|ColourLerp|GetLerpScriptC) "inOutQuad")
  ;[1 1 1] Create colour changing screen material
  (bind _returnvalue (Rendering|Material|CreateDynamicMaterialInstance "/Game/Material/ScreenMaterial.ScreenMaterial" "None" "None" :!class /Script/Engine.KismetMaterialLibrary))
  (bind _output_get (Variables|ColourLerp|SetScreenMaterialInstance _returnvalue))
  (Rendering|Material|SetMaterial (Variables|Default|GetCube) 0 _output_get))

(fn ConstructionScript)